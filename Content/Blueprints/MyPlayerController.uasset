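; MyPlayerController is a player controller that returns the player to the current checkpoint when R is pressed.
; It reads the CheckPoint actor from BP_ThirdPersonGameModeCustom and does nothing if none is valid.
; An existing character is moved to the checkpoint's rotation and slightly raised location; otherwise a new BP_ThirdPersonCharacterCustom is spawned there and possessed.
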(event EventBeginPlay)

(event EventTick
  (params (DeltaSeconds :type Float%20%28single-precision%29)))

(event Input|KeyboardEvents|R
  (params (Key :type Key%20Structure :default "None"))
  (bind _returnvalue (Game|GetPlayerCharacter 0))
  ;[0.15 0.15 0.15 0.5] Checkpoint
  (:Pressed
    (bind _asbp_third_person_game_mode_custom (Utilities|Casting|CastToBP_ThirdPersonGameModeCustom (Game|GetGameMode)))
    (bind _checkpoint (Variables|/Game/StealthGame/Core/GameModes/BP_ThirdPersonGameModeCustom.BP_ThirdPersonGameModeCustom_C|GetCheckPoint _asbp_third_person_game_mode_custom)
      (:then
        (if (Utilities|IsValid _returnvalue)
          (Transformation|SetActorLocationAndRotation _returnvalue (Math|Vector|MakeVector (.X (Math|Vector|BreakVector (Transformation|GetActorLocation _checkpoint))) (.Y (Math|Vector|BreakVector (Transformation|GetActorLocation _checkpoint))) (+ (.Z (Math|Vector|BreakVector (Transformation|GetActorLocation _checkpoint))) 5e+01)) (Transformation|GetActorRotation _checkpoint))
          (else
            (bind _returnvalue_2 (Game|SpawnActorfromClass "/Game/StealthGame/Core/Characters/PlayerCharacter/BP_ThirdPersonCharacterCustom.BP_ThirdPersonCharacterCustom_C" (Math|Transform|MakeTransform (Math|Vector|MakeVector (.X (Math|Vector|BreakVector (Transformation|GetActorLocation _checkpoint))) (.Y (Math|Vector|BreakVector (Transformation|GetActorLocation _checkpoint))) (+ (.Z (Math|Vector|BreakVector (Transformation|GetActorLocation _checkpoint))) 5e+01)) (Transformation|GetActorRotation _checkpoint) "1.000000,1.000000,1.000000") "Undefined" "MultiplyWithRoot" 0 0))
            (Pawn|Possess _returnvalue_2))))
      (:else))))

(fn ConstructionScript)