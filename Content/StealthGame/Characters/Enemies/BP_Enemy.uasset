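; Enemy actor for the stealth game that moves back and forth and is taken out when the player character runs into it.
; A Movement timeline drives the Body's relative Y position, while a Delay on its update toggles IsLooped to alternate between playing and reversing.
; Player overlap with the Capsule turns on Body physics, then after a short delay notifies the Manager to update its enemy count and destroys the actor.
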(event OnComponentBeginOverlap(Capsule)
  (params (OverlappedComponent :type Primitive%20Component%20Object%20Reference) (OtherActor :type Actor%20Object%20Reference) (OtherComp :type Primitive%20Component%20Object%20Reference) (OtherBodyIndex :type Integer) (bFromSweep :type Boolean) (SweepResult :type Hit%20Result%20Structure%20%28by%20ref%29))
  (Utilities|Casting|CastToBP_ThirdPersonCharacterCustom OtherActor)
  (Physics|SetSimulatePhysics (Variables|Default|GetBody) true)
  (Utilities|FlowControl|Delay 2.0)
  (Default|RemoveEnemyandCheck (Variables|Default|GetManager))
  (Actor|DestroyActor))

(event EventBeginPlay
  (bind _movement (Timeline|Movement Play) ; "Add Timeline" then double click to open Timeline\nthen create a Float Track and adjust nodes\nNow I move!
    (:Update
      (Transformation|SetRelativeLocation (Variables|Default|GetBody) (Math|Vector|MakeVector 0.0 _movement 0.0) false false) ; Split Location nodes and place in whichever (XYZ)\nI chose Y
      (Utilities|FlowControl|Delay 1.0) ; Change Duration time\nAdd Bollean in Variables (called IsLooped)\nCheck Default Value to Is Looped
      (if (Variables|Default|GetIsLooped) ; "If" statement
        (Variables|Default|SetIsLooped false) ; (Set Is Looped)\nIf true, no longer loops
        (Timeline|Movement Reverse)
        (else
          (Variables|Default|SetIsLooped true) ; If false, loops
          (Timeline|Movement Play))))))

(fn ConstructionScript)