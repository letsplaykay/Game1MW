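; BP_DoorEnd is a locked door, apparently the level's end door, that opens only for a player carrying enough keys.
; A box overlap casts to BP_ThirdPersonCharacterCustom and checks that its KeyCount is above a fixed threshold.
; On success, the DoorRotation timeline lerps the door mesh's yaw to swing it open; otherwise an on-screen locked message prints.
; Keys are not consumed, as the decrement logic is unconnected.
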(event OnComponentBeginOverlap(Boxcollision)
  (params (OverlappedComponent :type Primitive%20Component%20Object%20Reference) (OtherActor :type Actor%20Object%20Reference) (OtherComp :type Primitive%20Component%20Object%20Reference) (OtherBodyIndex :type Integer) (bFromSweep :type Boolean) (SweepResult :type Hit%20Result%20Structure%20%28by%20ref%29))
  (bind _relative_rotation (Variables|Default|GetRelative%20Rotation))
  (bind _asbp_third_person_character_custom (Utilities|Casting|CastToBP_ThirdPersonCharacterCustom OtherActor))
  (if (> (Variables|/Game/StealthGame/Core/Characters/PlayerCharacter/BP_ThirdPersonCharacterCustom.BP_ThirdPersonCharacterCustom_C|GetKey%20Count _asbp_third_person_character_custom) 3) ; Like an If Statement
    (bind _rotationrate (Timeline|DoorRotation Play)
      (:Update
        (Transformation|SetRelativeRotation (Variables|Default|GetSM_Door) (Math|Rotator|Lerp(Rotator) (Variables|Default|GetRelative%20Rotation) (Math|Rotator|CombineRotators (Math|Rotator|MakeRotator (.roll _relative_rotation) (.pitch _relative_rotation) (.yaw _relative_rotation)) (Math|Rotator|MakeRotator (.roll _relative_rotation) (.pitch _relative_rotation) -9e+01)) _rotationrate) false false)))
    (else
      (Development|PrintString "Get More Keys! Door is locked" true true "(R=0.479167,G=0.051103,B=0.000000,A=1.000000)" 5.0))))

(event Collision|EventActorBeginOverlap
  (params (OtherActor :type Actor%20Object%20Reference)))

(event EventTick
  (params (DeltaSeconds :type Float%20%28single-precision%29)))

(fn ConstructionScript)