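; BP_UnlockedDoor is a door in the stealth game that swings open, with no key check, when the player character enters its box trigger.
; The overlap plays an opening sound and runs a timeline that lerps the door mesh from its rotation saved at BeginPlay to a -90 degree yaw offset.
; There is no closing logic, and a leftover key-count branch is never executed.
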(event OnComponentBeginOverlap(Boxcollision)
  (params (OverlappedComponent :type Primitive%20Component%20Object%20Reference) (OtherActor :type Actor%20Object%20Reference) (OtherComp :type Primitive%20Component%20Object%20Reference) (OtherBodyIndex :type Integer) (bFromSweep :type Boolean) (SweepResult :type Hit%20Result%20Structure%20%28by%20ref%29))
  (bind _relative_rotation (Variables|Default|GetRelative%20Rotation))
  (Utilities|Casting|CastToBP_ThirdPersonCharacterCustom OtherActor)
  (Audio|PlaySoundatLocation "/Game/Developer/Audio/door_open2.door_open2" (Transformation|GetActorLocation) "0, 0, 0" 1.0 1.0 0.0 0 0 0 0)
  (bind _rotationrate (Timeline|DoorRotaiton Play)
    (:Update
      (Transformation|SetRelativeRotation (Variables|Default|GetSM_Door) (Math|Rotator|Lerp(Rotator) (Variables|Default|GetRelative%20Rotation) (Math|Rotator|CombineRotators (Math|Rotator|MakeRotator (.roll _relative_rotation) (.pitch _relative_rotation) (.yaw _relative_rotation)) (Math|Rotator|MakeRotator (.roll _relative_rotation) (.pitch _relative_rotation) -9e+01)) _rotationrate) false false))))

(event Collision|EventActorBeginOverlap
  (params (OtherActor :type Actor%20Object%20Reference)))

(event EventTick
  (params (DeltaSeconds :type Float%20%28single-precision%29)))

(event EventBeginPlay
  (Variables|Default|SetRelative%20Rotation (Variables|/Script/Engine.SceneComponent|GetRelativeRotation (Variables|Default|GetSM_Door))))

(fn ConstructionScript)